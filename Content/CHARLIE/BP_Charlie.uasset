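; Charlie is a companion pawn that moves between scripted story spots (kitchen, sofa, food, phone, ball) and fetches the player's ball.
; Externally callable events drive AIMoveTo toward ListaPosiciones actors, some playing mood sounds.
; Fetching attaches the ball and returns it to the player; later requests show rest dialogue, sending Charlie to unlock sofa interaction.
; Reaching the kitchen starts recursive random wandering, stopped by DesactivarMovimientoAleatorio.
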(event `self.ReceiveBeginPlay`
  (set `FloatingPawnMovement.MaxSpeed` 150.0 (`self.FloatingPawnMovement`))
  (bind _asbp_first_person_character (cast `/Game/FirstPerson/Blueprints/BP_FirstPersonCharacter` (`GameplayStatics.GetPlayerCharacter` 0)))
  (set `self.Rf Jugador` _asbp_first_person_character))

(event `self.ReceiveTick`
  (params (DeltaSeconds :type "Float (single-precision)")))

(event `BuscarPelota`
  (if (> (`self.NumeroVecesPelotaRecogida`) 0.0)
    (bind _returnvalue (`|CreateWidget` "/Game/FirstPerson/Widget/W_Dialogos.W_Dialogos_C" null "¿Cansado? ¿Nos tomamos un descanso?"))
    (`UserWidget.AddToViewport` _returnvalue 0)
    (`KismetSystemLibrary.Delay` 7.0)
    (`self.SubirAlSofa`)
    (elif (`KismetSystemLibrary.IsValid` (`self.Ref Pelota`))
      (`KismetSystemLibrary.PrintString` "Buscando pelota")
      (`PrimitiveComponent.SetSimulatePhysics` (`/Game/LevelPrototyping/Props_UVS/COMEDOR/PELOTA/BP_Pelota.Pelota` (`self.Ref Pelota`)) false)
      (`|AIMoveTo` self (`SceneComponent.K2_GetComponentLocation` (`/Game/LevelPrototyping/Props_UVS/COMEDOR/PELOTA/BP_Pelota.Pelota` (`self.Ref Pelota`))) null 1.0
        (:`OnSuccess`
          (`self.K2_AttachToActor` (`self.Ref Pelota`) self "None" "SnapToTarget" "SnapToTarget" "SnapToTarget" true)
          (`SceneComponent.K2_SetRelativeLocation` (`/Game/LevelPrototyping/Props_UVS/COMEDOR/PELOTA/BP_Pelota.Pelota` (`self.Ref Pelota`)) (`self.PosicionPelota`) false false)
          (`|AIMoveTo` self (0.0 0.0 0.0) (`self.Rf Jugador`) 150.0 true
            (:`OnSuccess`
              (`/Game/LevelPrototyping/Props_UVS/COMEDOR/PELOTA/BP_Pelota.Coger Pelota` (`self.Ref Pelota`))
              (set `self.NumeroVecesPelotaRecogida` (+ (`self.NumeroVecesPelotaRecogida`) 1.0)))))
        (:`OnFail`
          (`KismetSystemLibrary.PrintString` "Charlie a fallado en llegar a la pelota"))))))

(event `CaminarACocina`
  (bind _sonidos (`self.Sonidos`))
  (`KismetSystemLibrary.PrintString` "Moviendo a Charlie a la cocina")
  (`AudioComponent.Play` _sonidos 0.0)
  (`|AIMoveTo` self (`self.K2_GetActorLocation` (`|GetArrayItem` (`self.ListaPosiciones`))) null 1.0
    (:`OnSuccess`
      (`KismetSystemLibrary.Delay` 0.2)
      (`AudioComponent.Stop` _sonidos)
      (`self.MoverDeFormaRandom`))))

(event `MoverDeFormaRandom`
  (bind _desactivar_movimiento_aleatorio (`self.Desactivar movimiento Aleatorio`))
  (bind _sonidos (`self.Sonidos`))
  (`AudioComponent.SetSound` _sonidos "/Game/CHARLIE/SONIDOS/S_CharlieAsustado.S_CharlieAsustado")
  (`AudioComponent.Play` _sonidos 0.0)
  (bind _output_get (set `self.UbicacionRandom` (`NavigationSystemV1.K2_GetRandomReachablePointInRadius` (`self.K2_GetActorLocation`) 100.0 null null)))
  (`|AIMoveTo` self _output_get null 1.0
    (:`OnSuccess`
      (if _desactivar_movimiento_aleatorio
        (`KismetSystemLibrary.Delay` 3.0)
        (set `self.Desactivar movimiento Aleatorio` false)
        (else
          (`KismetSystemLibrary.Delay` 3.0)
          (`self.MoverDeFormaRandom`))))
    (:`OnFail`
      (if _desactivar_movimiento_aleatorio
        (set `self.Desactivar movimiento Aleatorio` false)
        (else
          (`KismetSystemLibrary.Delay` 3.0)
          (`self.MoverDeFormaRandom`))))))

(event `Comer`
  (bind _sonidos (`self.Sonidos`))
  (`AudioComponent.SetSound` _sonidos "/Game/CHARLIE/SONIDOS/S_CharlieRiendo.S_CharlieRiendo")
  (`AudioComponent.Play` _sonidos 0.0)
  (`|AIMoveTo` self (`self.K2_GetActorLocation` (`|GetArrayItem` (`self.ListaPosiciones`) 2)) null
    (:`OnSuccess`
      (`KismetSystemLibrary.PrintString` "Comiendo"))
    (:`OnFail`
      (`KismetSystemLibrary.PrintString` "Charlie fallo en ir a comer"))))

(event `CaminarATelefono`
  (bind _sonidos (`self.Sonidos`))
  (`AudioComponent.SetSound` _sonidos "/Game/CHARLIE/SONIDOS/S_CharlieAsustado.S_CharlieAsustado")
  (`AudioComponent.Play` _sonidos 0.0)
  (`|AIMoveTo` self (`self.K2_GetActorLocation` (`|GetArrayItem` (`self.ListaPosiciones`) 3)) null
    (:`OnSuccess`
      (`KismetSystemLibrary.PrintString` "Caminando a Telefono")
      (`AudioComponent.Play` (`self.Sonidos`) 0.0))
    (:`OnFail`
      (`KismetSystemLibrary.PrintString` "Charlie fallo en llegar al telefono"))))

(event `CaminarAPelota`
  (`|AIMoveTo` self (`self.K2_GetActorLocation` (`|GetArrayItem` (`self.ListaPosiciones`) 4)) null
    (:`OnSuccess`
      (`KismetSystemLibrary.PrintString` "Caminando a Pelota"))
    (:`OnFail`
      (`KismetSystemLibrary.PrintString` "Charlie fallo en llegar a la pelota"))))

(event `SubirAlSofa`
  (`|AIMoveTo` self (`self.K2_GetActorLocation` (`|GetArrayItem` (`self.ListaPosiciones`) 1)) null
    (:`OnSuccess`
      (`KismetSystemLibrary.Delay` 0.2)
      (`KismetSystemLibrary.PrintString` "Charlie se acurruca")
      (bind _returnvalue (`|CreateWidget` "/Game/FirstPerson/Widget/W_Dialogos.W_Dialogos_C" null "Deberia sentarme un poco también"))
      (`UserWidget.AddToViewport` _returnvalue 0)
      (set `/Game/LevelPrototyping/Blueprints/BP_Sofa.Se Puede Interactuar` true (`self.Ref Sofa`)))
    (:`OnFail`
      (`KismetSystemLibrary.PrintString` "Charlie a fallado en subir al sofa"))))

(fn `UserConstructionScript`)