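; BP_Musica_DIA is a music actor that plays a configurable track and fades it out after the sofa is interacted with.
; The construction script assigns the Musica variable to the Audio component.
; Tick polls the referenced Sofa's SofaInteractuado flag unless DIA4 is set, then waits on a Delay before a linear fade to silence.
; The check has no latch, so the delayed fade repeats while the flag stays true.
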(event `self.ReceiveBeginPlay`)

(event `self.ReceiveTick`
  (params (DeltaSeconds :type "Float (single-precision)"))
  (if (`self.DIA 4`)
    _
    (elif (or (`/Game/LevelPrototyping/Props_UVS/COMEDOR/SOFA/BP_Sofa.Sofa Interactuado` (`self.Sofa`)) false)
      (`KismetSystemLibrary.Delay` 10.0)
      (`AudioComponent.FadeOut` (`self.Audio`) 6.0 0.0 "Linear"))))

(fn `UserConstructionScript`
  (`AudioComponent.SetSound` (`self.Audio`) (`self.Musica`)))